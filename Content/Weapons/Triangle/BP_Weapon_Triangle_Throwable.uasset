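; Thrown triangle weapon that flies out from the player and returns like a boomerang.
; On BeginPlay it launches its physics mesh along the player's facing, and a fast looping timer applies constant acceleration back toward the player.
; After a short grace delay, overlapping the player destroys it and calls ShowWeapon on the character.
; The wall-stuck trace and movement-stop logic are disconnected.
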(event Collision|EventActorBeginOverlap
  (params (OtherActor :type Actor%20Object%20Reference))
  ;[0 0 0] Destroy if collided with player
  (if (Variables|Default|GetCanBeDestroyed)
    (bind _asbp_third_person_character (Utilities|Casting|CastToBP_ThirdPersonCharacter OtherActor))
    (Actor|DestroyActor)
    (Default|ShowWeapon _asbp_third_person_character)))

(event EventTick
  (params (DeltaSeconds :type Float%20%28single-precision%29))
  ;[0 0 0] Event Tick
)

(event EventBeginPlay
  ;[0 0 0] Set Destroyable after a delay
  (bind _asbp_third_person_character (Utilities|Casting|CastToBP_ThirdPersonCharacter (Game|GetPlayerCharacter 0)))
  (Variables|Default|SetThird%20Person%20Character _asbp_third_person_character)
  (CallFunction|StartProjectileMovement)
  (Utilities|FlowControl|Delay 0.2)
  (Variables|Default|SetCanBeDestroyed true))

(fn ConstructionScript)

(fn ProjectileMovement
  (if (< (Math|Float|Absolute(Float) (.x (Transformation|GetComponentVelocity (Variables|Default|GetTriangleMesh)))) 1e+02)
    _
    (else
      _))
  (Physics|AddForce (Variables|Default|GetTriangleMesh) (* (Math|Vector|GetUnitDirection(Vector) (Transformation|GetActorLocation) (Transformation|GetActorLocation (Variables|Default|GetThird%20Person%20Character))) 4.2e+02) "None" true))

(fn StartProjectileMovement
  (Physics|SetPhysicsLinearVelocity (Variables|Default|GetTriangleMesh) (* (Math|Vector|GetForwardVector (Transformation|GetActorRotation (Variables|Default|GetThird%20Person%20Character))) 3e+03) false "None")
  (bind _returnvalue (Utilities|Time|SetTimerbyFunctionName 0 "Projectile Movement" 0.001 true))
  (Variables|Default|SetProjectile%20Movement%20Timer%20Handle _returnvalue))