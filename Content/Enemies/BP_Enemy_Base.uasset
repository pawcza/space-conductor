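; Base enemy character providing combat actions, damage reaction, a patrol route getter and preset walk speeds.
; Montages drive attacking and weapon draw or sheathe, with notifies spawning or destroying a hand-socketed axe and completion firing dispatchers.
; ReportDamage stores hit data and raises an AI damage-sense event.
; Damaged applies attack-type knockback and reaction, blocking further hits until a notify restores vulnerability and clears the player's ignore entry.
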(event Custom|Damaged
  (bind _attack_type (Variables|Default|GetAttack%20Type))
  (Variables|Default|SetCanBeDamaged? false)
  (Physics|AddImpulse (Variables|Character|GetCharacterMovement) (* (Math|Vector|GetUnitDirection(Vector) (Math|Vector|MakeVector (.x (Transformation|GetActorLocation (Variables|Default|GetDamaging%20Actor))) 0.0 0.0) (Math|Vector|MakeVector (.x (Transformation|GetActorLocation)) 0.0 0.0)) (Utilities|Select :Index _attack_type :Option%200 0.0 :Option%201 7.5e+02 :Option%202 5e+02 :Option%203 1e+03)) true)
  (Animation|Montage|PlayMontage (Variables|Character|GetMesh) (Utilities|Select :Index _attack_type :Option%200 "/Game/Characters/Manny/Animations/Manny/Mixamo/MM_HitSmall_Montage.MM_HitSmall_Montage" :Option%201 "/Game/Characters/Manny/Animations/Manny/Mixamo/MM_HitSmall_Montage.MM_HitSmall_Montage" :Option%202 "/Game/Characters/Manny/Animations/Manny/Mixamo/MM_HitSmall_Montage.MM_HitSmall_Montage" :Option%203 "/Game/Characters/Manny/Animations/Manny/Mixamo/MM_HitBig_Montage.MM_HitBig_Montage")
    (:OnCompleted
      (Default|CallOnDamageFinished))
    (:OnNotifyBegin
      (Variables|Default|SetCanBeDamaged? true)
      (bind _asbp_third_person_character (Utilities|Casting|CastToBP_ThirdPersonCharacter (Game|GetPlayerCharacter 0)))
      (Utilities|Array|RemoveItem (Variables|/Game/ThirdPerson/Blueprints/BP_ThirdPersonCharacter.BP_ThirdPersonCharacter_C|GetIgnoredEnemies _asbp_third_person_character) self))))

(event Custom|Report%20Damage
  (params (Damaging%20Actor :type Actor%20Object%20Reference) (Damage%20Amount :type Float%20%28double-precision%29) (Damage%20Location :type Vector) (AttackType :type GameplayAbility_Attack_Type%20Enum :default "NewEnumerator3"))
  (if (Variables|Default|GetCanBeDamaged?)
    (Variables|Default|SetAttack%20Type AttackType)
    (bind _output_get (Variables|Default|SetDamaging%20Actor Damaging%20Actor))
    (bind _output_get_2 (Variables|Default|SetLastDamageLocation Damage%20Location))
    (Class|AISenseDamage|ReportDamageEvent self _output_get Damage%20Amount _output_get_2 "0, 0, 0" "None")))

(event Custom|Attack
  (Variables|Default|SetIsAttacking? true)
  (Animation|Montage|PlayMontage (Variables|Character|GetMesh) "/Game/Characters/Manny/Animations/Manny/Mixamo/MM_RightAttack_Montage.MM_RightAttack_Montage"
    (:OnCompleted
      (Default|CallOnAttackEnd)
      (Variables|Default|SetIsAttacking? false))))

(event Custom|WieldSword
  (Variables|Default|SetIsWieldingSword true)
  (bind _notifyname (Animation|Montage|PlayMontage (Variables|Character|GetMesh) "/Game/Characters/Manny/Animations/Manny/Mixamo/MM_WieldingSword_Montage.MM_WieldingSword_Montage")
    (:OnCompleted
      (Default|CallOnWieldSword))
    (:OnNotifyBegin
      (switch name _notifyname
        (:WieldSword
          (bind _returnvalue (Game|SpawnActorfromClass "/Game/Weapons/BP_Enemy_Axe.BP_Enemy_Axe_C" (Transformation|GetActorTransform) "Undefined" "MultiplyWithRoot" 0 0))
          (Variables|Default|SetSwordActor _returnvalue)
          (Transformation|AttachComponentToComponent _returnvalue (Variables|Character|GetMesh) "hand_r_Weapon" "SnapToTarget" "SnapToTarget" "SnapToTarget" true))))))

(event Custom|SheathWeapon
  (bind _notifyname (Animation|Montage|PlayMontage (Variables|Character|GetMesh) "/Game/Characters/Manny/Animations/Manny/Mixamo/MM_SheathingSword_Montage.MM_SheathingSword_Montage")
    (:OnCompleted
      (Default|CallOnSheathSword))
    (:OnNotifyBegin
      (switch name _notifyname
        (:SheathSword
          (Actor|DestroyActor (Variables|Default|GetSwordActor))
          (Variables|Default|SetIsWieldingSword false))))))

(fn ConstructionScript)

(fn HandleHit)

(fn GetPatrolRoute
  (return (Variables|AI|GetPatrolRoute)))

(fn SetMovementSpeed
  (params (Speed :type E_MovementSpeedEnum%20Enum :default "NewEnumerator0"))
  (bind _output_get (Variables|/Script/Engine.CharacterMovementComponent|SetMaxWalkSpeed (Variables|Character|GetCharacterMovement) (Utilities|Select :Index Speed :NewEnumerator0 0.0 :NewEnumerator1 1e+02 :NewEnumerator4 2.5e+02 :NewEnumerator2 3e+02)))
  (return _output_get))